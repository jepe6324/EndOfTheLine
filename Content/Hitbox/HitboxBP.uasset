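; HitboxBP is a melee attack hitbox actor that notifies whatever its HitboxDisplay component overlaps.
; SpawnHitbox switches on HitboxType, then applies HitboxMaterial to HitboxDisplay and moves it to HitboxLocation.
; On begin overlap, the component sends EnemyMeleeAttackMessage to the other actor without any filtering.
; A node that would make the display visible is left unconnected and never runs.
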(event `SpawnHitbox`
  (switch `EHitboxEnum` (`self.hitboxType`)
    (:`BH_STRIKE`
      (`PrimitiveComponent.SetMaterial` (`self.HitboxDisplay`) 0 "/Game/Hitbox/HitboxMaterial.HitboxMaterial")
      (`SceneComponent.K2_SetWorldLocation` (`self.HitboxDisplay`) (`self.hitboxLocation`) false false))))

(event `self.HitboxDisplay.OnComponentBeginOverlap`
  (params (OverlappedComponent :type "PrimitiveComponent Object Reference") (OtherActor :type "Actor Object Reference") (OtherComp :type "PrimitiveComponent Object Reference") (OtherBodyIndex :type Integer) (bFromSweep :type Boolean) (SweepResult :type "HitResult Structure (by ref)"))
  (message `/Game/GameMode/Game_BPI.EnemyMeleeAttack` OtherActor))

(fn `UserConstructionScript`)