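; BP_Button is a UI button that syncs keyboard focus with mouse hover and restyles itself to match.
; Start sets a looping timer that polls CheckFocus instead of binding hover or focus events.
; CheckFocus gives a hovered button keyboard focus and the ButtonStyle look.
; Otherwise it applies KeyPressed or KeyNotPressed styles depending on whether the button holds keyboard focus.
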(fn `CheckFocus`
  (if (`self.IsHovered`)
    (`self.SetKeyboardFocus`)
    (`self.SetStyle` (`self.ButtonStyle`))
    (else
      (`self.SetStyle` (select `bool` (`self.HasKeyboardFocus`) :`false` (`self.KeyNotPressed`) :`true` (`self.KeyPressed`))))))

(fn `Start`
  (`KismetSystemLibrary.K2_SetTimer` null "CheckFocus" 0.1 true))